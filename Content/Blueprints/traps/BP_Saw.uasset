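; BP_Saw is a moving saw trap that kills the third-person character on hit and expires after a configurable lifespan.
; After a start delay, a Timeline rotates PivotMesh through a near-full turn and replays itself on finish for continuous motion.
; Tick shifts PivotMesh in world space by a non-zero Direction each frame, without delta-time scaling.
; A hit on the Saw component calls Die on the character.
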(event OnComponentHit(saw)
  (params (HitComponent :type Primitive%20Component%20Object%20Reference) (OtherActor :type Actor%20Object%20Reference) (OtherComp :type Primitive%20Component%20Object%20Reference) (NormalImpulse :type Vector :default "0, 0, 0") (Hit :type Hit%20Result%20Structure%20%28by%20ref%29))
  (bind _asbp_third_person_character (Utilities|Casting|CastToBP_ThirdPersonCharacter OtherActor))
  (Default|Die _asbp_third_person_character))

(event Custom|Replay
  (bind _newtrack_0 (Timeline|Timeline PlayFromStart)
    (:Update
      (Transformation|SetRelativeRotation (Variables|Default|GetPivotMesh) (Math|Rotator|Lerp(Rotator) "0, 0, 0" "0.000000,359.000000,0.000000" _newtrack_0) false false))
    (:Finished
      (CallFunction|Replay))))

(event EventBeginPlay
  (Actor|SetLifeSpan (Variables|Default|GetduréeDeVieDeLaScie))
  (Utilities|FlowControl|Delay (Variables|Default|GetDuration))
  (bind _newtrack_0 (Timeline|Timeline Play)
    (:Update
      (Transformation|SetRelativeRotation (Variables|Default|GetPivotMesh) (Math|Rotator|Lerp(Rotator) "0, 0, 0" "0.000000,359.000000,0.000000" _newtrack_0) false false))
    (:Finished
      (CallFunction|Replay))))

(event Collision|EventActorBeginOverlap
  (params (OtherActor :type Actor%20Object%20Reference)))

(event EventTick
  (params (DeltaSeconds :type Float%20%28single-precision%29))
  (if (not (Utilities|Operators|EqualEqual :A (Variables|Default|Getdirection)))
    (Class|SceneComponent|AddWorldTransform (Variables|Default|GetPivotMesh) (Math|Transform|MakeTransform (Variables|Default|Getdirection) "0, 0, 0" "1.000000,1.000000,1.000000") false false)))

(fn ConstructionScript)