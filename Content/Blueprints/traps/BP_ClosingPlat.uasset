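; BP_ClosingPlat is a looping trap whose moving plate opens and closes, killing the player character on contact with its trigger Box.
; On BeginPlay, a double-speed Timeline lerps PlateauMouvant from its initial relative location to the local origin while rotating it from a quarter-turn to zero.
; Each finish flips the Timeline direction, creating an endless ping-pong.
; Any BP_ThirdPersonCharacter overlapping the Box calls Die, regardless of the plate's position.
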(event OnComponentBeginOverlap(Box)
  (params (OverlappedComponent :type Primitive%20Component%20Object%20Reference) (OtherActor :type Actor%20Object%20Reference) (OtherComp :type Primitive%20Component%20Object%20Reference) (OtherBodyIndex :type Integer) (bFromSweep :type Boolean) (SweepResult :type Hit%20Result%20Structure%20%28by%20ref%29))
  (bind _asbp_third_person_character (Utilities|Casting|CastToBP_ThirdPersonCharacter OtherActor))
  (Default|Die _asbp_third_person_character))

(event Custom|backward
  (bind (_direction _newtrack_0) (Timeline|Timeline ReverseFromEnd)
    (:Update
      (Transformation|SetRelativeLocation (Variables|Default|GetplateauMouvant) (Math|Vector|Lerp(Vector) (Variables|Default|GetReturn%20Value%20Location) "0, 0, 0" _newtrack_0) false false)
      (Transformation|SetRelativeRotation (Variables|Default|GetplateauMouvant) (Math|Rotator|Lerp(Rotator) "-90.000000,0.000000,0.000000" "0, 0, 0" _newtrack_0) false false))
    (:Finished
      (switch Utilities|FlowControl|Switch|SwitchonETimelineDirection _direction
        (:Forward
          (CallFunction|Backward))
        (:Backward
          (CallFunction|Forward))))))

(event Custom|forward
  (bind (_direction _newtrack_0) (Timeline|Timeline PlayFromStart)
    (:Update
      (Transformation|SetRelativeLocation (Variables|Default|GetplateauMouvant) (Math|Vector|Lerp(Vector) (Variables|Default|GetReturn%20Value%20Location) "0, 0, 0" _newtrack_0) false false)
      (Transformation|SetRelativeRotation (Variables|Default|GetplateauMouvant) (Math|Rotator|Lerp(Rotator) "-90.000000,0.000000,0.000000" "0, 0, 0" _newtrack_0) false false))
    (:Finished
      (switch Utilities|FlowControl|Switch|SwitchonETimelineDirection _direction
        (:Forward
          (CallFunction|Backward))
        (:Backward
          (CallFunction|Forward))))))

(event EventBeginPlay
  (bind _plateaumouvant (Variables|Default|GetplateauMouvant))
  (bind _returnvalue (Transformation|GetRelativeTransform _plateaumouvant))
  (Components|Timeline|SetPlayRate (Variables|Default|GetTimeline) 2.0)
  (Variables|Default|SetReturn%20Value%20Location (.location _returnvalue))
  (Variables|Default|SetReturn%20Value%20Rotation (.rotation _returnvalue))
  (bind (_direction _newtrack_0) (Timeline|Timeline Play)
    (:Update
      (Transformation|SetRelativeLocation (Variables|Default|GetplateauMouvant) (Math|Vector|Lerp(Vector) (Variables|Default|GetReturn%20Value%20Location) "0, 0, 0" _newtrack_0) false false)
      (Transformation|SetRelativeRotation (Variables|Default|GetplateauMouvant) (Math|Rotator|Lerp(Rotator) "-90.000000,0.000000,0.000000" "0, 0, 0" _newtrack_0) false false))
    (:Finished
      (switch Utilities|FlowControl|Switch|SwitchonETimelineDirection _direction
        (:Forward
          (CallFunction|Backward))
        (:Backward
          (CallFunction|Forward))))))

(fn ConstructionScript)